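; BP_EndlessRunnerGameState is the endless runner's game state Blueprint, managing the main UI across play and death.
; On BeginPlay it creates and stores the HUD and pause menu widgets, adding the HUD to the viewport and calling CloseMenu on the pause menu.
; The OnDeath event calls SaveHighScore, removes the HUD and shows a newly created GameOver widget.
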(event EventBeginPlay
  (Utilities|FlowControl|Sequence
    (:then_0
      (bind _returnvalue (UserInterface|CreateWidget "/Game/LevelAssets/UI/WBP_HUD.WBP_HUD_C"))
      (bind _output_get (Variables|Default|SetHUD _returnvalue))
      (UserInterface|Viewport|AddtoViewport _output_get 0))
    (:then_1
      (bind _returnvalue_2 (UserInterface|CreateWidget "/Game/LevelAssets/UI/PauseMenu.PauseMenu_C"))
      (bind _output_get_2 (Variables|Default|SetPauseMenu _returnvalue_2))
      (Default|CloseMenu _output_get_2))))

(event EventTick
  (params (DeltaSeconds :type Float%20%28single-precision%29)))

(event EventOnDeath
  (params (PlayerIndex :type Integer))
  (Class|EndlessRunnerGameState|SaveHighScore)
  (Widget|RemovefromParent (Variables|Default|GetHUD))
  (bind _returnvalue (UserInterface|CreateWidget "/Game/LevelAssets/UI/GameOver.GameOver_C"))
  (UserInterface|Viewport|AddtoViewport _returnvalue 0))

(fn ConstructionScript)